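; BP_SwitchButton is a one-shot pressure switch that opens a linked door when a component tagged Player overlaps its box.
; A timeline animates the button mesh's height, then on finish opens TargetDoor and marks both door and switch as finished.
; The SetEventFinished override calls its parent, sets the mesh to its relative origin and disables the box's collision, preventing further overlaps.
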(event OnComponentBeginOverlap(Box)
  (params (OverlappedComponent :type Primitive%20Component%20Object%20Reference) (OtherActor :type Actor%20Object%20Reference) (OtherComp :type Primitive%20Component%20Object%20Reference) (OtherBodyIndex :type Integer) (bFromSweep :type Boolean) (SweepResult :type Hit%20Result%20Structure%20%28by%20ref%29))
  (if (Components|ComponentHasTag OtherComp "Player")
    (bind _buttonz (Timeline|SwitchOn Play)
      (:Update
        (Transformation|SetRelativeLocation (Variables|Default|GetSTM_Button) (Math|Vector|MakeVector 0.0 0.0 _buttonz) false false))
      (:Finished
        (Utilities|FlowControl|Sequence
          (:then_0
            (bind _targetdoor (Variables|Default|GetTargetDoor)
              (:then
                (Default|OpenDoor _targetdoor))
              (:else)))
          (:then_1
            (bind _targetdoor_2 (Variables|Default|GetTargetDoor)
              (:then
                (CallFunction|SetEventFinished _targetdoor_2))
              (:else)))
          (:then_2
            (CallFunction|SetEventFinished)))))))

(event EventBeginPlay
  (|CallParentFunction))

(fn ConstructionScript)

(fn SetEventFinished
  (|CallParentFunction)
  (Transformation|SetRelativeLocation (Variables|Default|GetSTM_Button) "0, 0, 0" false false)
  (Collision|SetCollisionEnabled (Variables|Default|GetBox) "NoCollision"))