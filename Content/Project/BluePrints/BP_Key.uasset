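; BP_Key is a key pickup actor that records its collection in the game instance.
; When a component overlaps its sphere and passes a tag check (tag left as None), it notifies the player through ACOverlapPlayer using Keyname and saves that key's status via MyGameInstance.
; It then calls SetEventFinished, an override that runs the parent's finish logic and destroys the actor.
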(event OnComponentBeginOverlap(Sphere)
  (params (OverlappedComponent :type Primitive%20Component%20Object%20Reference) (OtherActor :type Actor%20Object%20Reference) (OtherComp :type Primitive%20Component%20Object%20Reference) (OtherBodyIndex :type Integer) (bFromSweep :type Boolean) (SweepResult :type Hit%20Result%20Structure%20%28by%20ref%29))
  (if (Components|ComponentHasTag OtherComp "None")
    (Default|NotifytoPlayer (Variables|Default|GetAC_OverlapPlayer) OtherActor (Variables|Default|GetKeyname))
    (Default|SaveKeyStatus (Variables|Default|GetMyGameInstance) (Variables|Default|GetKeyname) "NewEnumerator1")
    (CallFunction|SetEventFinished)))

(event EventBeginPlay
  (|CallParentFunction))

(fn ConstructionScript)

(fn SetEventFinished
  (|CallParentFunction)
  (Actor|DestroyActor))